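; BP_DeerStag is a deer stag animal whose AI reacts to the player and to damage.
; Pawn sensing of the player or taking any damage sets the HasSeenPlayer blackboard key on its AI controller.
; PlayerFound raises movement from walking to running speed, while PlayerLost restores walking speed and clears the key.
; Neither event is called within this Blueprint.
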(event `self.ReceiveBeginPlay`
  (set `CharacterMovementComponent.MaxWalkSpeed` 100.0 (`self.CharacterMovement`)))

(event `self.PawnSensing.OnSeePawn`
  (params (Pawn :type "Pawn Object Reference"))
  (if (== Pawn (`GameplayStatics.GetPlayerPawn` 0))
    (`BlackboardComponent.SetValueAsBool` (`AIBlueprintHelperLibrary.GetBlackboard` (`AIBlueprintHelperLibrary.GetAIController` self)) (`self.HasSeenPlayer?`) true)))

(event `/Game/Animals/Interface/BI_PlayerSeen.PlayerFound`
  (set `CharacterMovementComponent.MaxWalkSpeed` 600.0 (`self.CharacterMovement`)))

(event `/Game/Animals/Interface/BI_PlayerSeen.PlayerLost`
  (set `CharacterMovementComponent.MaxWalkSpeed` 100.0 (`self.CharacterMovement`))
  (`BlackboardComponent.SetValueAsBool` (`AIBlueprintHelperLibrary.GetBlackboard` (`AIBlueprintHelperLibrary.GetAIController` self)) (`self.HasSeenPlayer?`) false))

(event `self.ReceiveAnyDamage`
  (params (Damage :type "Float (single-precision)") (DamageType :type "DamageType Object Reference") (InstigatedBy :type "Controller Object Reference") (DamageCauser :type "Actor Object Reference"))
  (`BlackboardComponent.SetValueAsBool` (`AIBlueprintHelperLibrary.GetBlackboard` (`AIBlueprintHelperLibrary.GetAIController` self)) (`self.HasSeenPlayer?`) true))

(fn `UserConstructionScript`)