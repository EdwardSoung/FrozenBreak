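; Fox animal Blueprint that drives an AI controller blackboard and switches walk speed with its behavior state.
; Pawn sensing sets HasSeenPlayer, while PlayerFound and PlayerLost change speed, the latter also clearing the flag.
; Attack starts a montage and immediately damages player zero with a hard-coded value, without a hit check.
; OnHalfHealth raises speed and sets TimeToRun once, guarded by NeedRunning.
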(event `self.ReceiveBeginPlay`
  (set `CharacterMovementComponent.MaxWalkSpeed` 100.0 (`self.CharacterMovement`))
  (set `self.AnimalDamage` 10.0))

(event `/Game/Animals/Interface/BI_PlayerSeen.PlayerFound`
  (set `CharacterMovementComponent.MaxWalkSpeed` 700.0 (`self.CharacterMovement`)))

(event `/Game/Animals/Interface/BI_PlayerSeen.PlayerLost`
  (set `CharacterMovementComponent.MaxWalkSpeed` 100.0 (`self.CharacterMovement`))
  (`BlackboardComponent.SetValueAsBool` (`AIBlueprintHelperLibrary.GetBlackboard` (`AIBlueprintHelperLibrary.GetAIController` self)) (`self.HasSeenPlayer?`) false))

(event `self.PawnSensing.OnSeePawn`
  (params (Pawn :type "Pawn Object Reference"))
  (`BlackboardComponent.SetValueAsBool` (`AIBlueprintHelperLibrary.GetBlackboard` (`AIBlueprintHelperLibrary.GetAIController` self)) (`self.HasSeenPlayer?`) true))

(event `/Game/Animals/Interface/BPI_Attack.Attack`
  (`|PlayMontage` (`self.Mesh`) "/Game/Animals/Fox/Animations/AM_Attack.AM_Attack"
    (:`then`
      (`GameplayStatics.ApplyDamage` (`GameplayStatics.GetPlayerPawn` 0) 10.0))))

(event `self.OnHalfHealth`
  (if (not (`self.NeedRunning`))
    (set `CharacterMovementComponent.MaxWalkSpeed` 600.0 (`self.CharacterMovement`))
    (`BlackboardComponent.SetValueAsBool` (`AIBlueprintHelperLibrary.GetBlackboard` (`AIBlueprintHelperLibrary.GetAIController` self)) (`self.TimeToRun`) true)
    (set `self.NeedRunning` true)))

(fn `UserConstructionScript`)