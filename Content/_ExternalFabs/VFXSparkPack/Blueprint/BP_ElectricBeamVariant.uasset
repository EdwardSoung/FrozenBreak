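; Electric spark VFX actor that periodically shoots up to three beam arcs at random nearby surfaces.
; A looping timer, its interval randomized once at BeginPlay, calls ShootArc to fire three events, the latter two after short random delays.
; Each moves a dummy target within its radius range and line-traces to it.
; Hits set the beam endpoint, spawn an impact emitter and briefly flash a light; misses collapse the beam and deactivate the particle component.
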(event `self.ReceiveBeginPlay`
  ;[1 1 1] link to function
  (`KismetSystemLibrary.K2_SetTimer` null "ShootArc" (`KismetMathLibrary.RandomFloatInRange` (`self.Beam Time Min`) (`self.Beam Time Max`)) true))

(event `CE_ShootArc`
  (bind _returnvalue (`SceneComponent.K2_GetComponentLocation` (`self.VFX_BeamTest`)))
  ;[1 1 1] Beam1
  (`ParticleSystemComponent.SetBeamSourcePoint` 0 _returnvalue 1)
  (bind _output_get (set `self.NewVar0` (* (`KismetMathLibrary.RandomUnitVector`) (`KismetMathLibrary.RandomFloatInRange` (`self.Beam Radius 1 Min`) (`self.Beam Radius 1 Max`)))))
  (`SceneComponent.K2_SetRelativeLocation` (`self.DummyTarget`) _output_get false false)
  (bind (_outhit _returnvalue_2) (`KismetSystemLibrary.LineTraceSingle` _returnvalue (`SceneComponent.K2_GetComponentLocation` (`self.DummyTarget`)) "TraceTypeQuery1"))
  (if _returnvalue_2
    (bind (_bblockinghit _binitialoverlap _time _distance _location _impactpoint _normal) (`GameplayStatics.BreakHitResult` _outhit))
    (`ParticleSystemComponent.SetBeamTargetPoint` 0 _location 1)
    (`GameplayStatics.SpawnEmitterAtLocation` "/Game/_ExternalFabs/VFXSparkPack/Particles/VFX_ElectricBeamHit.VFX_ElectricBeamHit" _location (`KismetMathLibrary.MakeRotationFromAxes` _normal))
    (`SceneComponent.SetVisibility` (`self.LightOn`))
    (`SceneComponent.K2_SetWorldLocation` _location)
    (`KismetSystemLibrary.RetriggerableDelay` 0.2)
    (`SceneComponent.SetVisibility` (`self.LightOff`))
    (else
      (`ParticleSystemComponent.SetBeamTargetPoint` 0 (`SceneComponent.K2_GetComponentLocation` (`self.VFX_BeamTest`)) 1)
      (`ActorComponent.Deactivate` (`self.VFX_BeamTest`))
      (`SceneComponent.SetVisibility` (`self.LightOff`)))))

(event `CE_ShootArc2`
  (bind _returnvalue (`SceneComponent.K2_GetComponentLocation` (`self.VFX_BeamTest`)))
  ;[1 1 1] beam2
  (`KismetSystemLibrary.RetriggerableDelay` (`KismetMathLibrary.RandomFloatInRange` 0.3 0.5))
  (`ParticleSystemComponent.SetBeamSourcePoint` 1 _returnvalue 1)
  (bind _output_get (set `self.NewVar0` (* (`KismetMathLibrary.RandomUnitVector`) (`KismetMathLibrary.RandomFloatInRange` (`self.Beam Radius 2 Min`) (`self.Beam Radius 2 Max`)))))
  (`SceneComponent.K2_SetRelativeLocation` (`self.DummyTarget`) _output_get false false)
  (bind (_outhit _returnvalue_2) (`KismetSystemLibrary.LineTraceSingle` _returnvalue (`SceneComponent.K2_GetComponentLocation` (`self.DummyTarget`)) "TraceTypeQuery1"))
  (if _returnvalue_2
    (bind (_bblockinghit _binitialoverlap _time _distance _location _impactpoint _normal) (`GameplayStatics.BreakHitResult` _outhit))
    (`ParticleSystemComponent.SetBeamTargetPoint` 1 _location 1)
    (`GameplayStatics.SpawnEmitterAtLocation` "/Game/_ExternalFabs/VFXSparkPack/Particles/VFX_ElectricBeamHit.VFX_ElectricBeamHit" _location (`KismetMathLibrary.MakeRotationFromAxes` _normal))
    (`SceneComponent.SetVisibility` (`self.LightOn`))
    (`SceneComponent.K2_SetWorldLocation` _location)
    (`KismetSystemLibrary.RetriggerableDelay` 0.2)
    (`SceneComponent.SetVisibility` (`self.LightOff`))
    (else
      (`ParticleSystemComponent.SetBeamTargetPoint` 1 (`SceneComponent.K2_GetComponentLocation` (`self.VFX_BeamTest`)) 1)
      (`ActorComponent.Deactivate` (`self.VFX_BeamTest`))
      (`SceneComponent.SetVisibility` (`self.LightOff`)))))

(event `CE_shootArc3`
  (bind _returnvalue (`SceneComponent.K2_GetComponentLocation` (`self.VFX_BeamTest`)))
  ;[1 1 1] beam3
  (`KismetSystemLibrary.RetriggerableDelay` (`KismetMathLibrary.RandomFloatInRange` 0.3 0.5))
  (`ParticleSystemComponent.SetBeamSourcePoint` 2 _returnvalue 1)
  (bind _output_get (set `self.NewVar0` (* (`KismetMathLibrary.RandomUnitVector`) (`KismetMathLibrary.RandomFloatInRange` (`self.Beam Radius 3 Min`) (`self.Beam Radius 3 Max`)))))
  (`SceneComponent.K2_SetRelativeLocation` (`self.DummyTarget`) _output_get false false)
  (bind (_outhit _returnvalue_2) (`KismetSystemLibrary.LineTraceSingle` _returnvalue (`SceneComponent.K2_GetComponentLocation` (`self.DummyTarget`)) "TraceTypeQuery1"))
  (if _returnvalue_2
    (bind (_bblockinghit _binitialoverlap _time _distance _location _impactpoint _normal) (`GameplayStatics.BreakHitResult` _outhit))
    (`ParticleSystemComponent.SetBeamTargetPoint` 2 _location 1)
    (`GameplayStatics.SpawnEmitterAtLocation` "/Game/_ExternalFabs/VFXSparkPack/Particles/VFX_ElectricBeamHit.VFX_ElectricBeamHit" _location (`KismetMathLibrary.MakeRotationFromAxes` _normal))
    (`SceneComponent.SetVisibility` (`self.LightOn`))
    (`SceneComponent.K2_SetWorldLocation` _location)
    (`KismetSystemLibrary.RetriggerableDelay` 0.2)
    (`SceneComponent.SetVisibility` (`self.LightOff`))
    (else
      (`ParticleSystemComponent.SetBeamTargetPoint` 2 (`SceneComponent.K2_GetComponentLocation` (`self.VFX_BeamTest`)) 1)
      (`ActorComponent.Deactivate` (`self.VFX_BeamTest`))
      (`SceneComponent.SetVisibility` (`self.LightOff`)))))

(fn `ShootArc`
  (`self.CE_ShootArc`)
  (`self.CE_ShootArc2`)
  (`self.CE_shootArc3`))

(fn `UserConstructionScript`)