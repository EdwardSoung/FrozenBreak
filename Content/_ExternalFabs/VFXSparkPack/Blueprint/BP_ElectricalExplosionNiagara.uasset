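; Looping electrical explosion VFX actor that pairs Niagara systems with point lights and sound cues.
; Construction script pushes exposed color, intensity, radius, shadow, light-function and spark settings into both lights and both Niagara systems.
; BeginPlay runs pre-explosion sparks for a random delay, swaps to the explosion burst with its light and sound, then waits and restarts the cycle through LoopMe.
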(event `self.ReceiveBeginPlay`
  ;[1 1 1] Pre explosion time zaps
  (`ActorComponent.Activate` (`self.NS_ElectricalPreExplosion`) true :!label _label)
  (`SceneComponent.SetVisibility` (`self.ElectPreExpLight`) (`self.LightOn`) false)
  (`AudioComponent.Play` (`self.Fire_Sparks01_Cue`) 0.0)
  (`KismetSystemLibrary.Delay` (`KismetMathLibrary.RandomFloatInRange` (`self.Delay Min time`) (`self.Delay Max Time`)))
  (`ActorComponent.Deactivate` (`self.NS_ElectricalPreExplosion`))
  (`SceneComponent.SetVisibility` (`self.ElectPreExpLight`) (`self.LightOff`) false)
  (`ActorComponent.Deactivate` (`self.Fire_Sparks01_Cue`))
  ;[1 1 1] Explosion light and sound
  (`ActorComponent.Activate` (`self.NS_ElectricalExplosion`) true)
  (`SceneComponent.SetVisibility` (`self.ElecExpLight`) (`self.LightOn`) false)
  (`AudioComponent.Play` (`self.Reflections_Spark_Cue`) 0.0)
  (`KismetSystemLibrary.Delay` (`KismetMathLibrary.RandomFloatInRange` 1.0 2.0))
  (`SceneComponent.SetVisibility` (`self.ElecExpLight`) (`self.LightOff`) false)
  (`KismetSystemLibrary.Delay` 3.0)
  (`self.LoopMe`))

(event `LoopMe`
  (goto _label))

(fn `UserConstructionScript`
  (bind _elecexplight (`self.ElecExpLight`))
  (bind _electpreexplight (`self.ElectPreExpLight`))
  (bind _ns_electricalexplosion (`self.NS_ElectricalExplosion`))
  (bind _ns_electricalpreexplosion (`self.NS_ElectricalPreExplosion`))
  ;[1 1 1] Pre Explosion Light Settings
  (`LightComponent.SetLightColor` _electpreexplight (`self.Pre Light Color`) true)
  (`LightComponent.SetIntensity` _electpreexplight (`self.Pre Light Intensity`))
  (`LocalLightComponent.SetAttenuationRadius` _electpreexplight (`self.Pre Light Attenuation Radius`))
  (`LightComponentBase.SetCastShadows` _electpreexplight (`self.Cast Shadows`))
  (`SceneComponent.K2_AddRelativeLocation` _electpreexplight (`self.Pre Light Source`) false false)
  (`LightComponent.SetLightFunctionMaterial` _electpreexplight (`self.Pre Light Function Material`))
  ;[1 1 1] Explosion Light Settings
  (`LightComponent.SetLightColor` _elecexplight (`self.Exp Light color`) true)
  (`LightComponent.SetIntensity` _elecexplight (`self.Light Intensity`))
  (`LocalLightComponent.SetAttenuationRadius` _elecexplight (`self.Attenuation Radius`))
  (`LightComponentBase.SetCastShadows` _elecexplight (`self.Cast Shadows`))
  (`SceneComponent.K2_AddRelativeLocation` _elecexplight (`self.Point Light Loc`) false false)
  (`LightComponent.SetLightFunctionMaterial` _elecexplight (`self.Explosion Light Function Material`))
  ;[1 1 1] Explosion Niagara Settings
  (`FXSystemComponent.SetColorParameter` _ns_electricalexplosion "SmokeColor" (`self.Explosion Smoke Color`))
  (`FXSystemComponent.SetColorParameter` _ns_electricalexplosion "SparkStartColor" (`self.Spark Start Color`))
  (`FXSystemComponent.SetColorParameter` _ns_electricalexplosion "SparkEndColor" (`self.Explosion Spart End Color`))
  (`FXSystemComponent.SetFloatParameter` _ns_electricalexplosion "SparkLerpOffset" (`self.Spark Lerp Offset`))
  (`FXSystemComponent.SetFloatParameter` _ns_electricalexplosion "SparkScaleAlpha" (`self.Spark Alpha Scale`))
  (`FXSystemComponent.SetFloatParameter` _ns_electricalexplosion "SparkScaleColor" (`self.Spark Color Scale`))
  ;[1 1 1] Pre Explosion Niagara Settings
  (`FXSystemComponent.SetColorParameter` _ns_electricalpreexplosion "PreSmokeColor" (`self.Pre-Smoke Color`))
  (`FXSystemComponent.SetColorParameter` _ns_electricalpreexplosion "PreSparkStartColor" (`self.Pre Spark Start Color`))
  (`FXSystemComponent.SetColorParameter` _ns_electricalpreexplosion "PreSparkEndColor" (`self.Pre Spark End Color`))
  (`FXSystemComponent.SetFloatParameter` _ns_electricalpreexplosion "PreSparkLerpOffset" (`self.Pre Spark Lerp Offset`))
  (`FXSystemComponent.SetFloatParameter` _ns_electricalpreexplosion "PreSparkScaleAlpha" (`self.Pre Spark Alpah Multiploer`))
  (`FXSystemComponent.SetFloatParameter` _ns_electricalpreexplosion "PreSparkScaleColor" (`self.Pre Spark color Multiplier`)))