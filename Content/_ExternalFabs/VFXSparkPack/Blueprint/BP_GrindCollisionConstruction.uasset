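; Grinding spark effect actor that turns sparks, smoke and a light on while it touches a surface.
; Each Tick, a short downward sphere trace toggles the effect and light, aligning the particles to the hit normal.
; A DoOnce starts playback once per contact and resets when contact is lost, which also stops it.
; The construction script applies the exposed collision radius, light settings and particle color parameters.
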(event `self.ReceiveTick`
  (params (DeltaSeconds :type "Float (single-precision)"))
  (bind _returnvalue (`SceneComponent.K2_GetComponentLocation`))
  (bind (_outhit _returnvalue_2) (`KismetSystemLibrary.SphereTraceSingleForObjects` _returnvalue (+ _returnvalue (0.0 0.0 -20.0)) (`self.CollisionSphere`) (`|MakeArray` "ObjectTypeQuery1" "ObjectTypeQuery2" "ObjectTypeQuery3" "ObjectTypeQuery4" "ObjectTypeQuery5" "ObjectTypeQuery6" :!type "EObjectTypeQuery Enum") true))
  (if _returnvalue_2
    (`SceneComponent.K2_SetWorldRotation` (`self.VFX_GrindNoLight`) (`KismetMathLibrary.MakeRotationFromAxes` (`.Normal` (`GameplayStatics.BreakHitResult` _outhit))) false false)
    (`ActorComponent.Activate` false)
    (`SceneComponent.SetVisibility` (`self.LightOn`))
    (`|DoOnceMultiInput` :!label _label
      (:`A Out`
        (`AudioComponent.Play` 0.0)))
    (else
      (`|ExecutionSequence`
        (:`then_0`
          (goto _label :!via `Reset In`))
        (:`then_1`
          (`ActorComponent.Deactivate`)
          (`SceneComponent.SetVisibility` (`self.LightOff`))
          (`AudioComponent.Stop`))))))

(fn `UserConstructionScript`
  (bind _vfx_grindnolight (`self.VFX_GrindNoLight`))
  (bind _light_grind (`self.Light_Grind`))
  ;[1 1 1] Collision Settings
  (`SphereComponent.SetSphereRadius` (`self.GrindCollision`) (`self.CollisionSphere`) true)
  ;[1 1 1] Light Settings
  (`LightComponent.SetLightColor` _light_grind (`self.Light Color`) true)
  (`LightComponent.SetIntensity` _light_grind (`self.Light Intensity`))
  (`LocalLightComponent.SetAttenuationRadius` _light_grind (`self.Light Attenuation Radius`))
  (`LightComponentBase.SetCastShadows` _light_grind (`self.Light Cast Shadows`))
  (`SceneComponent.K2_AddRelativeLocation` _light_grind (`self.Light Location`) false false)
  (`LightComponent.SetLightFunctionMaterial` _light_grind (`self.Light Function`))
  ;[1 1 1] color settings
  (`ParticleSystemComponent.SetColorParameter` _vfx_grindnolight "SparkColor" (`self.Effect Color`))
  (`ParticleSystemComponent.SetFloatParameter` _vfx_grindnolight "SparkColorScale" (`self.Color Intensity`))
  (`ParticleSystemComponent.SetFloatParameter` _vfx_grindnolight "SparkAlphaScale" (`self.Alpha Intensity`))
  (`ParticleSystemComponent.SetColorParameter` _vfx_grindnolight "SmokeColor" (`self.SmokeColor`))
  (`ParticleSystemComponent.SetFloatParameter` _vfx_grindnolight "SmokeColorScale" (`self.Smoke Color Scale`))
  (`ParticleSystemComponent.SetFloatParameter` _vfx_grindnolight "SmokeAlphaScale" (`self.Smoke Alpha Scale`)))