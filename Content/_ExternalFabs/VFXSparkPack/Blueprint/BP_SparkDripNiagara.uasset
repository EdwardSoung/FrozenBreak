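; BP_SparkDripNiagara is an intermittent dripping-spark effect combining a Niagara system with a light.
; The construction script applies exposed light settings, including a light function material, and pushes spark and smoke colors, scales and randomized alphas into Niagara parameters.
; From BeginPlay, an endless loop alternates random-length active and idle periods, toggling the particles, visibility and playback on and off.
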(event `self.ReceiveBeginPlay`
  (bind _niagarasparkdrip (`self.NiagaraSparkDrip`))
  (`ActorComponent.ToggleActive` _niagarasparkdrip :!label _label)
  (`SceneComponent.ToggleVisibility` false)
  (`AudioComponent.Play` 0.0)
  (`KismetSystemLibrary.Delay` (`KismetMathLibrary.RandomFloatInRange` (`self.SparkDrip Active Min`) (`self.SparkDrip Active Max`)))
  (`ActorComponent.Deactivate` _niagarasparkdrip)
  (`SceneComponent.ToggleVisibility` false)
  (`AudioComponent.Stop`)
  (`KismetSystemLibrary.Delay` (`KismetMathLibrary.RandomFloatInRange` (`self.SparkDrip Dealy Min`) (`self.SparkDrip Dealy Max`)))
  (`self.OnLoop`))

(event `OnLoop`
  (goto _label))

(fn `UserConstructionScript`
  (bind _light_sparkdrip (`self.Light SparkDrip`))
  (bind _niagarasparkdrip (`self.NiagaraSparkDrip`))
  ;[1 1 1] Light Settings
  (`LightComponent.SetLightColor` _light_sparkdrip (`self.Light Color`) true)
  (`LightComponent.SetIntensity` _light_sparkdrip (`self.Light Intensity`))
  (`LocalLightComponent.SetAttenuationRadius` _light_sparkdrip (`self.Attenuation Radius`))
  (`LightComponentBase.SetCastShadows` _light_sparkdrip (`self.Cast Shadows`))
  (`SceneComponent.K2_AddRelativeLocation` _light_sparkdrip (`self.Point Light Loc`) false false)
  (`LightComponent.SetLightFunctionMaterial` _light_sparkdrip (`self.Light Function Material`))
  ;[1 1 1] Effect color Settings
  (`ParticleSystemComponent.SetColorParameter` _niagarasparkdrip "SparkColor" (`self.Spark Color`))
  (`ParticleSystemComponent.SetFloatParameter` _niagarasparkdrip "SparkColorScale" (`self.SparkIntensity`))
  (`ParticleSystemComponent.SetFloatParameter` _niagarasparkdrip "SparkAlphaScale" (`KismetMathLibrary.RandomFloatInRange` (`self.Spark Alpha Intensity Min`) (`self.Spark Alpha Intensity Max`)))
  (`ParticleSystemComponent.SetColorParameter` _niagarasparkdrip "SmokeColor" (`self.Smoke Color`))
  (`ParticleSystemComponent.SetFloatParameter` _niagarasparkdrip "SmokeColorScale" (`self.Smoke Color Intensity`))
  (`ParticleSystemComponent.SetFloatParameter` _niagarasparkdrip "SmokeAlphaScale" (`KismetMathLibrary.RandomFloatInRange` (`self.Smoke Alpha Scale Min`) (`self.Smoke Alpha Scale Max`))))